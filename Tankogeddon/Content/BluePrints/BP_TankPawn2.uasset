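; Tank pawn Blueprint that drives the player's HUD and game-over screen.
; BeginPlay creates both widgets for player controller 0 and keeps the game-over widget hidden.
; Tick polls TankController's IsDead, revealing game-over on death and otherwise pushing ammo and HealthComponent health to the HUD.
; The ammo value is a stored variable, written through SetAmmoState.
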(event `self.ReceiveBeginPlay`
  ;[1 1 1] Create and hide gameover widget
  (bind _returnvalue (`|CreateWidget` "/Game/BluePrints/Widgets/WBP_GameOver.WBP_GameOver_C" (`GameplayStatics.GetPlayerController` 0)))
  (bind _output_get (set `self.GameOverWidget` _returnvalue))
  (`UserWidget.AddToViewport` _output_get 0)
  (`Widget.SetVisibility` (`self.GameOverWidget`) "Hidden")
  ;[1 1 1] Create HUD widget
  (bind _returnvalue_2 (`|CreateWidget` "/Game/BluePrints/Widgets/WBP_HUD.WBP_HUD_C" (`GameplayStatics.GetPlayerController` 0)))
  (bind _output_get_2 (set `self.HUDwidget` _returnvalue_2))
  (`UserWidget.AddToViewport` _output_get_2 0))

(event `self.ReceiveTick`
  (params (DeltaSeconds :type "Float (single-precision)"))
  ;[1 1 1] Check if tank alive
  (bind _astank_controller (cast `TankController` (`GameplayStatics.GetPlayerController` 0)))
  (bind _returnvalue (`TankController.isDead` _astank_controller))
  (if _returnvalue
    ;[1 1 1] Show gameover widget if tank dead
    (`Widget.SetVisibility` (`self.GameOverWidget`) "Visible")
    (else
      ;[1 1 1] Update health and ammo in HUD
      (bind _aswbp_hud (cast `/Game/BluePrints/Widgets/WBP_HUD` (`self.HUDwidget`)))
      (`/Game/BluePrints/Widgets/WBP_HUD.SetAmmoCount` _aswbp_hud (`self.AmmoState`))
      (bind _aswbp_hud_2 (cast `/Game/BluePrints/Widgets/WBP_HUD` (`self.HUDwidget`)))
      (`/Game/BluePrints/Widgets/WBP_HUD.SetHealthState` _aswbp_hud_2 (`HealthComponent.GetHealthState` (`self.HealthComponent`))))))

(fn `SetAmmoState`
  (params (AmmoState :type Text))
  (set `self.AmmoState` AmmoState))

(fn `UserConstructionScript`)